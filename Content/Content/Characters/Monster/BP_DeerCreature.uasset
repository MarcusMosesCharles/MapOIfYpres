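; BP_DeerCreature is a deer creature that endlessly patrols a looping route of waypoints.
; BeginPlay caches the locations of the PointsObject actors into a Destinations array and resets the index.
; Tick re-issues AIMoveTo toward the current destination until StopLoop is set on arrival.
; After a pause, the index advances with modulo wraparound, prints for debugging and movement resumes.
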(event `self.ReceiveBeginPlay`
  (for _array_element (`self.PointsObject`)
    (bind _output_get (set `self.TempVector` (`self.K2_GetActorLocation` _array_element)))
    (`KismetArrayLibrary.Array_Set` (`self.Destinations`) (`self.Counter`) _output_get true)
    (bind _result (`/Engine/EditorBlueprintResources/StandardMacros.IncrementInt` (`self.Counter`))
      (:`  `
        (set `self.Counter` _result))))
  (`self.ResetCoutner`))

(event `ResetCoutner`
  (set `self.Counter` 0))

(event `self.ReceiveTick`
  (params (DeltaSeconds :type "Float (single-precision)"))
  (if (not (`self.StopLoop`))
    (`|AIMoveTo` self (`|GetArrayItem` (`self.Destinations`) (`self.Counter`)) null 0.1 true
      (:`OnSuccess`
        (set `self.StopLoop` true)
        (`KismetSystemLibrary.Delay` 4.0)
        (`self.MoveToNextPoint`)))))

(event `MoveToNextPoint`
  (bind _result (`/Engine/EditorBlueprintResources/StandardMacros.IncrementInt` (`self.Counter`))
    (:`  `
      (set `self.Counter` (`KismetMathLibrary.Conv_Int64ToInt` (mod (`KismetMathLibrary.Conv_IntToInt64` _result) (`KismetMathLibrary.Conv_IntToInt64` (`KismetArrayLibrary.Array_Length` (`self.Destinations`))))))
      (`KismetSystemLibrary.PrintText` (`KismetTextLibrary.Conv_IntToText` (`self.Counter`)))
      (set `self.StopLoop` false))))

(fn `UserConstructionScript`)