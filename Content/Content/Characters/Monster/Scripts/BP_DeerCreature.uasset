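; BP_DeerCreature is a monster character that prepares a list of destination points and reacts to seeing the player.
; On BeginPlay it stores the locations of MonsterPoints-tagged actors, sets a slow walk speed, and makes its capsule ignore NPCIgnoreObstacle-tagged actors when moving.
; When PawnSensing spots BP_ThirdPersonCharacter, it sets the PlayerDetected blackboard key and raises the detection alpha in its animation blueprint.
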(event `self.ReceiveBeginPlay`
  (bind _outactors (`GameplayStatics.GetAllActorsWithTag` "MonsterPoints"))
  (for _array_element _outactors
    (bind _output_get (set `self.TempVector` (`self.K2_GetActorLocation` _array_element)))
    (`KismetArrayLibrary.Array_Set` (`self.Destinations`) (`self.Counter`) _output_get true)
    (bind _result (`/Engine/EditorBlueprintResources/StandardMacros.IncrementInt` (`self.Counter`))
      (:`  `
        (set `self.Counter` _result)
        (set `CharacterMovementComponent.MaxWalkSpeed` 100.0 (`self.CharacterMovement`))
        (bind _outactors_2 (`GameplayStatics.GetAllActorsWithTag` "NPCIgnoreObstacle"))
        (for _array_element_2 _outactors_2
          (`PrimitiveComponent.IgnoreActorWhenMoving` (`self.CapsuleComponent`) _array_element_2 true)))))
  (`self.ResetCoutner`))

(event `ResetCoutner`
  (set `self.Counter` 0))

(event `self.PawnSensing.OnSeePawn`
  (params (Pawn :type "Pawn Object Reference"))
  (cast `/Game/ThirdPerson/Blueprints/BP_ThirdPersonCharacter` Pawn)
  (`BlackboardComponent.SetValueAsBool` (`AIBlueprintHelperLibrary.GetBlackboard` (`AIBlueprintHelperLibrary.GetAIController` self)) "PlayerDetected" true)
  (bind _asabp_deer_creature (cast `/Game/Content/Characters/Monster/Animations/ABP_DeerCreature` (`SkeletalMeshComponent.GetAnimInstance` (`self.Mesh`))))
  (set `/Game/Content/Characters/Monster/Animations/ABP_DeerCreature.PlayerDetectedAlpha` 1.0 _asabp_deer_creature))

(fn `UserConstructionScript`)