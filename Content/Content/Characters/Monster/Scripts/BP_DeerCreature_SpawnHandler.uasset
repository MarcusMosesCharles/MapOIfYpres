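; BP_DeerCreature_SpawnHandler spawns a single deer creature at a random tagged point in the level.
; On BeginPlay it stores the location of every actor tagged DeerSpawn in MovementPointsLocations.
; It then picks one stored location at random and spawns BP_DeerCreature there as an AI pawn, with a small upward offset.
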(event `self.ReceiveBeginPlay`
  (bind _movementpointslocations (`self.MovementPointsLocations`))
  (bind _outactors (`GameplayStatics.GetAllActorsWithTag` "DeerSpawn"))
  (for _array_element _outactors
    (`KismetArrayLibrary.Array_Add` (`self.MovementPointsLocations`) (`self.K2_GetActorLocation` _array_element)))
  (`AIBlueprintHelperLibrary.SpawnAIFromClass` "/Game/Content/Characters/Monster/Scripts/BP_DeerCreature.BP_DeerCreature_C" null (+ (`|GetArrayItem` _movementpointslocations (`KismetMathLibrary.RandomIntegerInRange` 0 (- (`KismetArrayLibrary.Array_Length` _movementpointslocations) 1))) (0.0 0.0 100.0)) (struct) false null))

(fn `UserConstructionScript`)