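; BP_TriggerWalk is a trigger volume that flags when the deer creature is inside it, for use by that creature's AI.
; Its Box component's begin and end overlap events respond only to BP_DeerCreature actors.
; They set the WalkTriggered bool on that creature's AI controller blackboard to true on entry and false on exit.
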(event `self.Box.OnComponentBeginOverlap`
  (params (OverlappedComponent :type "PrimitiveComponent Object Reference") (OtherActor :type "Actor Object Reference") (OtherComp :type "PrimitiveComponent Object Reference") (OtherBodyIndex :type Integer) (bFromSweep :type Boolean) (SweepResult :type "HitResult Structure (by ref)"))
  (bind _asbp_deer_creature (cast `/Game/Content/Characters/Monster/Scripts/BP_DeerCreature` OtherActor))
  (`BlackboardComponent.SetValueAsBool` (`AIBlueprintHelperLibrary.GetBlackboard` (`AIBlueprintHelperLibrary.GetAIController` _asbp_deer_creature)) "WalkTriggered" true))

(event `self.Box.OnComponentEndOverlap`
  (params (OverlappedComponent :type "PrimitiveComponent Object Reference") (OtherActor :type "Actor Object Reference") (OtherComp :type "PrimitiveComponent Object Reference") (OtherBodyIndex :type Integer))
  (bind _asbp_deer_creature (cast `/Game/Content/Characters/Monster/Scripts/BP_DeerCreature` OtherActor))
  (`BlackboardComponent.SetValueAsBool` (`AIBlueprintHelperLibrary.GetBlackboard` (`AIBlueprintHelperLibrary.GetAIController` _asbp_deer_creature)) "WalkTriggered" false))

(fn `UserConstructionScript`)