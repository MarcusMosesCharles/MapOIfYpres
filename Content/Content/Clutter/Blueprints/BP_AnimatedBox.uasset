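; BP_AnimatedBox is an interactable army box that plays open and close animations on its skeletal mesh.
; Overlapping InteractionCollision registers the box as BP_ThirdPersonCharacter's CurrentInteractable; Interact plays the open animation if BoxIsOpen is false, but never sets that flag true.
; Any actor ending overlap plays the close animation and resets the flag; for the character, it also clears CurrentInteractable.
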(event `self.InteractionCollision.OnComponentBeginOverlap`
  (params (OverlappedComponent :type "PrimitiveComponent Object Reference") (OtherActor :type "Actor Object Reference") (OtherComp :type "PrimitiveComponent Object Reference") (OtherBodyIndex :type Integer) (bFromSweep :type Boolean) (SweepResult :type "HitResult Structure (by ref)"))
  (bind _asbp_third_person_character (cast `/Game/ThirdPerson/Blueprints/BP_ThirdPersonCharacter` OtherActor))
  (set `/Game/ThirdPerson/Blueprints/BP_ThirdPersonCharacter.CurrentInteractable` self _asbp_third_person_character)
  (`KismetSystemLibrary.PrintString` "Player is near, box is interactable"))

(event `/Game/ThirdPerson/Input/BPI_Interactable.Interact`
  (if (not (`self.BoxIsOpen`))
    (`SkeletalMeshComponent.PlayAnimation` (`self.SkeletalMesh`) "/Game/Content/Clutter/Interior/Animations/ArmyBox-Animation-Open.ArmyBox-Animation-Open" false)))

(event `self.InteractionCollision.OnComponentEndOverlap`
  (params (OverlappedComponent :type "PrimitiveComponent Object Reference") (OtherActor :type "Actor Object Reference") (OtherComp :type "PrimitiveComponent Object Reference") (OtherBodyIndex :type Integer))
  (`SkeletalMeshComponent.PlayAnimation` (`self.SkeletalMesh`) "/Game/Content/Clutter/Interior/Animations/ArmyBox-Animation-Close.ArmyBox-Animation-Close" false)
  (set `self.BoxIsOpen` false)
  (bind _asbp_third_person_character (cast `/Game/ThirdPerson/Blueprints/BP_ThirdPersonCharacter` OtherActor))
  (set `/Game/ThirdPerson/Blueprints/BP_ThirdPersonCharacter.CurrentInteractable` null _asbp_third_person_character)
  (`KismetSystemLibrary.PrintString` "Player moved away, box is not interactable"))

(fn `UserConstructionScript`)