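; BP_DoorCollider is an interactable door spot that the player can board up with carried planks.
; Overlapping its collider while holding a plank registers it as the character's current interactable and shows a prompt widget, both cleared on exit.
; Interacting detaches the held plank, snaps it to the first of four attach points, removes that point from the available list and clears the holding flag.
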(event `self.ReceiveBeginPlay`
  ;[1 1 1] Populate the attach points array on begin play
  (set `self.AvailableAttachPoints` (`|MakeArray` (`self.PlankAttachPoint`) (`self.PlankAttachPoint1`) (`self.PlankAttachPoint2`) (`self.PlankAttachPoint3`))))

(event `self.InteractionCollider.OnComponentBeginOverlap`
  (params (OverlappedComponent :type "PrimitiveComponent Object Reference") (OtherActor :type "Actor Object Reference") (OtherComp :type "PrimitiveComponent Object Reference") (OtherBodyIndex :type Integer) (bFromSweep :type Boolean) (SweepResult :type "HitResult Structure (by ref)"))
  ;[1 1 1] Player approaches door
  (bind _asbp_third_person_character (cast `/Game/ThirdPerson/Blueprints/BP_ThirdPersonCharacter` OtherActor))
  (if (`/Game/ThirdPerson/Blueprints/BP_ThirdPersonCharacter.IsHoldingPlank` _asbp_third_person_character)
    (set `/Game/ThirdPerson/Blueprints/BP_ThirdPersonCharacter.CurrentInteractable` self _asbp_third_person_character) ; Set current interactable to the window
    (bind _aswb_interact_prompt (cast `/Game/Blueprints/WB_InteractPrompt` (`WidgetComponent.GetUserWidgetObject` (`self.InteractWidget`))))
    (`Widget.SetVisibility` _aswb_interact_prompt "Visible") ; Display interact message
    (set `/Game/Blueprints/WB_InteractPrompt.MessageFromObject` (`self.InteractMessage`) _aswb_interact_prompt)
    (`KismetSystemLibrary.PrintString` "player can board up door")))

(event `self.Interact`
  (bind _output (`|GetArrayItem` (`self.AvailableAttachPoints`)))
  ;[1 1 1] Player interacts with window (only available if they are holding the plank)
  (bind _asbp_third_person_character (cast `/Game/ThirdPerson/Blueprints/BP_ThirdPersonCharacter` (`GameplayStatics.GetPlayerCharacter` 0)))
  (if (> (`KismetArrayLibrary.Array_Length` (`self.AvailableAttachPoints`)) 0)
    (bind _heldobject (`/Game/ThirdPerson/Blueprints/BP_ThirdPersonCharacter.HeldObject` _asbp_third_person_character))
    (`self.K2_DetachFromActor` _heldobject "KeepWorld" "KeepWorld" "KeepWorld") ; Detach the held object (plank) from the player
    (`self.K2_SetActorLocationAndRotation` _heldobject (`SceneComponent.K2_GetComponentLocation` _output) (`SceneComponent.K2_GetComponentRotation` _output) false false) ; Set the plank transforms to the attach point values
    (`KismetArrayLibrary.Array_Remove` (`self.AvailableAttachPoints`))
    (set `/Game/ThirdPerson/Blueprints/BP_ThirdPersonCharacter.IsHoldingPlank` false _asbp_third_person_character) ; Set IsHoldingPlank = false
  ))

(event `self.InteractionCollider.OnComponentEndOverlap`
  (params (OverlappedComponent :type "PrimitiveComponent Object Reference") (OtherActor :type "Actor Object Reference") (OtherComp :type "PrimitiveComponent Object Reference") (OtherBodyIndex :type Integer))
  ;[1 1 1] Player moves away from window
  (bind _asbp_third_person_character (cast `/Game/ThirdPerson/Blueprints/BP_ThirdPersonCharacter` OtherActor))
  (set `/Game/ThirdPerson/Blueprints/BP_ThirdPersonCharacter.CurrentInteractable` null _asbp_third_person_character) ; Set current interactable = NULL
  (bind _aswb_interact_prompt (cast `/Game/Blueprints/WB_InteractPrompt` (`WidgetComponent.GetUserWidgetObject` (`self.InteractWidget`))))
  (`Widget.SetVisibility` _aswb_interact_prompt "Hidden") ; Hide the interact message
)

(fn `UserConstructionScript`)