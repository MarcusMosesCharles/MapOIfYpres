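; BP_WindowCollider2 is an interactable window that the player boards up with a carried plank.
; Overlapping InteractionCollider while holding the plank sets the window as the character's CurrentInteractable and shows its WB_InteractPrompt message; leaving clears both.
; Interact detaches the held plank, snaps it to PlankAttachPoint, clears the holding state and interactable, then plays hammering audio while briefly disabling player input via a fixed delay.
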(event `self.InteractionCollider.OnComponentBeginOverlap`
  (params (OverlappedComponent :type "PrimitiveComponent Object Reference") (OtherActor :type "Actor Object Reference") (OtherComp :type "PrimitiveComponent Object Reference") (OtherBodyIndex :type Integer) (bFromSweep :type Boolean) (SweepResult :type "HitResult Structure (by ref)"))
  ;[1 1 1] Player approaches window
  (bind _asbp_third_person_character (cast `/Game/ThirdPerson/Blueprints/BP_ThirdPersonCharacter` OtherActor))
  (if (`/Game/ThirdPerson/Blueprints/BP_ThirdPersonCharacter.IsHoldingPlank` _asbp_third_person_character)
    (set `/Game/ThirdPerson/Blueprints/BP_ThirdPersonCharacter.CurrentInteractable` self _asbp_third_person_character) ; Set current interactable to the window
    (bind _aswb_interact_prompt (cast `/Game/Blueprints/WB_InteractPrompt` (`WidgetComponent.GetUserWidgetObject` (`self.InteractWidget`))))
    (`Widget.SetVisibility` _aswb_interact_prompt "Visible") ; Display interact message
    (set `/Game/Blueprints/WB_InteractPrompt.MessageFromObject` (`self.InteractMessage`) _aswb_interact_prompt)))

(event `self.Interact`
  (bind _plankattachpoint (`self.PlankAttachPoint`))
  ;[1 1 1] Player interacts with window (only available if they are holding the plank)
  (bind _asbp_third_person_character (cast `/Game/ThirdPerson/Blueprints/BP_ThirdPersonCharacter` (`GameplayStatics.GetPlayerCharacter` 0)))
  (bind _heldobject (`/Game/ThirdPerson/Blueprints/BP_ThirdPersonCharacter.HeldObject` _asbp_third_person_character))
  (`self.K2_DetachFromActor` _heldobject "KeepWorld" "KeepWorld" "KeepWorld") ; Detach the held object (plank) from the player
  (`self.K2_SetActorLocationAndRotation` _heldobject (`SceneComponent.K2_GetComponentLocation` _plankattachpoint) (`SceneComponent.K2_GetComponentRotation` _plankattachpoint) false false) ; Set the plank transforms to the attach point values
  (set `/Game/ThirdPerson/Blueprints/BP_ThirdPersonCharacter.IsHoldingPlank` false _asbp_third_person_character) ; Set IsHoldingPlank = false
  (set `/Game/ThirdPerson/Blueprints/BP_ThirdPersonCharacter.CurrentInteractable` null _asbp_third_person_character) ; Reset current interactable
  ;;[1 1 1] Play audio clip & disable movement until it completes
  (`AudioComponent.Play` (`self.HammeringNoise`) 0.0)
  (`/Game/ThirdPerson/Blueprints/BP_ThirdPersonCharacter.DisableInputs` _asbp_third_person_character)
  (`KismetSystemLibrary.Delay` 1.5)
  (`/Game/ThirdPerson/Blueprints/BP_ThirdPersonCharacter.EnableInputs` _asbp_third_person_character))

(event `self.InteractionCollider.OnComponentEndOverlap`
  (params (OverlappedComponent :type "PrimitiveComponent Object Reference") (OtherActor :type "Actor Object Reference") (OtherComp :type "PrimitiveComponent Object Reference") (OtherBodyIndex :type Integer))
  ;[1 1 1] Player moves away from window
  (bind _asbp_third_person_character (cast `/Game/ThirdPerson/Blueprints/BP_ThirdPersonCharacter` OtherActor))
  (set `/Game/ThirdPerson/Blueprints/BP_ThirdPersonCharacter.CurrentInteractable` null _asbp_third_person_character) ; Set current interactable = NULL
  (bind _aswb_interact_prompt (cast `/Game/Blueprints/WB_InteractPrompt` (`WidgetComponent.GetUserWidgetObject` (`self.InteractWidget`))))
  (`Widget.SetVisibility` _aswb_interact_prompt "Hidden") ; Hide the interact message
)

(fn `UserConstructionScript`)