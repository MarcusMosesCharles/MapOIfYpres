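; Ambient forest sound handler that periodically plays monster screams, crow calls or owl calls at points in the level.
; BeginPlay caches every actor tagged MonsterEventLocation as a sound spot.
; Tick feeds a random 15–30 second Delay, which acts as a repeating timer.
; A looping random MultiGate then picks one of the three sounds and plays it at a randomly chosen spot's location.
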(event `self.ReceiveBeginPlay`
  (bind _outactors (`GameplayStatics.GetAllActorsWithTag` "MonsterEventLocation"))
  (set `self.SoundSpots` _outactors))

(event `self.ReceiveTick`
  (params (DeltaSeconds :type "Float (single-precision)"))
  (bind _soundspots (`self.SoundSpots`))
  (bind _returnvalue (`self.K2_GetActorLocation` (`|GetArrayItem` _soundspots (`KismetMathLibrary.RandomIntegerInRange` 0 (- (`KismetArrayLibrary.Array_Length` _soundspots) 1)))))
  (`KismetSystemLibrary.Delay` (`KismetMathLibrary.Conv_IntToDouble` (`KismetMathLibrary.RandomIntegerInRange` 15 30)))
  (`|MultiGate` true true
    (:`Out 0`
      (`GameplayStatics.PlaySoundAtLocation` "/Game/Content/Audio/Ambience/Monster/Ambience/Screams/MonsterScreams.MonsterScreams" _returnvalue (struct) 1.0 1.0 0.0 null null null null))
    (:`Out 1`
      (`GameplayStatics.PlaySoundAtLocation` "/Game/Content/Audio/Ambience/Animal/crow4_Cue.crow4_Cue" _returnvalue (struct) 1.0 1.0 0.0 null null null null))
    (:`Out 2`
      (`GameplayStatics.PlaySoundAtLocation` "/Game/Content/Audio/Ambience/Animal/owl4_Cue.owl4_Cue" _returnvalue (struct) 1.0 1.0 0.0 null null null null))))

(fn `UserConstructionScript`)